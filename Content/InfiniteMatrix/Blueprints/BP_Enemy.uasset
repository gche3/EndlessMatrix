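; BP_Enemy is an enemy actor that damages the player on contact and awards score when hit by a projectile.
; On spawn it sets its lifespan inversely proportional to the player's forward speed, so it expires sooner when the player moves faster.
; Mesh overlap with the player reduces health and destroys the enemy.
; Overlap with a projectile destroys the enemy, adds to the player's score and updates the stats UI.
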(event `self.ReceiveBeginPlay`
  (bind _asbp_player (cast `/Game/InfiniteMatrix/Blueprints/BP_Player` (`GameplayStatics.GetPlayerPawn` 0)))
  (`self.SetLifeSpan` (/ 7500.0 (`/Game/InfiniteMatrix/Blueprints/BP_Player.ForwardSpeed` _asbp_player))))

(event `self.StaticMeshComponent.OnComponentBeginOverlap`
  (params (OverlappedComponent :type "PrimitiveComponent Object Reference") (OtherActor :type "Actor Object Reference") (OtherComp :type "PrimitiveComponent Object Reference") (OtherBodyIndex :type Integer) (bFromSweep :type Boolean) (SweepResult :type "HitResult Structure (by ref)"))
  (bind _asbp_player (cast `/Game/InfiniteMatrix/Blueprints/BP_Player` OtherActor)
    (:`then`
      (`/Game/InfiniteMatrix/Blueprints/BP_Player.UpdateHealth` _asbp_player -5.0)
      (`self.K2_DestroyActor`))
    (:`CastFailed`
      (cast `/Game/InfiniteMatrix/Blueprints/BP_Projectile` OtherActor)
      (`self.K2_DestroyActor`)
      (bind _asbp_player_2 (cast `/Game/InfiniteMatrix/Blueprints/BP_Player` (`GameplayStatics.GetPlayerPawn` 0)))
      (set `/Game/InfiniteMatrix/Blueprints/BP_Player.Score` (+ 5 (`/Game/InfiniteMatrix/Blueprints/BP_Player.Score` _asbp_player_2)) _asbp_player_2)
      (`/Game/InfiniteMatrix/UI/WBP_Stats.UpdateScore` (`/Game/InfiniteMatrix/Blueprints/BP_Player.StatsUI` _asbp_player_2) (`/Game/InfiniteMatrix/Blueprints/BP_Player.Score` _asbp_player_2)))))

(fn `UserConstructionScript`)