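; BP_Health_Pac is a health pickup actor that restores health to BP_Player on overlap, then destroys itself.
; It spins continuously on all three axes in Tick.
; On BeginPlay it sets its lifespan inversely to the player's ForwardSpeed, so missed pickups expire sooner as the player moves faster.
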(event `self.ReceiveBeginPlay`
  (bind _asbp_player (cast `/Game/InfiniteMatrix/Blueprints/BP_Player` (`GameplayStatics.GetPlayerPawn` 0)))
  (`self.SetLifeSpan` (/ 7500.0 (`/Game/InfiniteMatrix/Blueprints/BP_Player.ForwardSpeed` _asbp_player))))

(event `self.ReceiveTick`
  (params (DeltaSeconds :type "Float (single-precision)"))
  (bind _returnvalue (* DeltaSeconds 25.0))
  (`SceneComponent.K2_AddLocalRotation` (`self.RootComponent`) (`KismetMathLibrary.MakeRotator` _returnvalue _returnvalue _returnvalue) false false))

(event `self.RootComponent.OnComponentBeginOverlap`
  (params (OverlappedComponent :type "PrimitiveComponent Object Reference") (OtherActor :type "Actor Object Reference") (OtherComp :type "PrimitiveComponent Object Reference") (OtherBodyIndex :type Integer) (bFromSweep :type Boolean) (SweepResult :type "HitResult Structure (by ref)"))
  (bind _asbp_player (cast `/Game/InfiniteMatrix/Blueprints/BP_Player` OtherActor))
  (`/Game/InfiniteMatrix/Blueprints/BP_Player.UpdateHealth` _asbp_player 10.0)
  (`self.K2_DestroyActor`))

(fn `UserConstructionScript`)